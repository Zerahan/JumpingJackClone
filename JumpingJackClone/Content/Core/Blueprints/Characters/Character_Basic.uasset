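; Basic character Blueprint that shows a HUD widget while possessed by a player controller and flickers while recovering from damage.
; BeginPlay puts a dynamic material on the Mesh and Cube, and the recovery event toggles its IsFlickering parameter.
; The construction script sizes both from the capsule half height and lowers the Mesh by that amount.
; Overlap and hit events only forward to the parent class.
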(event Custom|OnRecovering
  (params (IsRecovering :type Boolean))
  (Rendering|Material|SetScalarParameterValue (Variables|Default|GetDynamicMaterial) "IsFlickering" (select IsRecovering 1.0 0.0) :!class /Script/Engine.MaterialInstanceDynamic))

(event EventBeginPlay
  (bind _returnvalue (Rendering|Material|CreateDynamicMaterialInstance "/Game/Core/Materials/TestCharacter_Mat.TestCharacter_Mat" "TestCharacter" "None" :!class /Script/Engine.KismetMaterialLibrary))
  (Variables|Default|SetDynamicMaterial _returnvalue)
  (Rendering|Material|SetMaterial (Variables|Character|GetMesh) 0 (Variables|Default|GetDynamicMaterial))
  (EventDispatchers|BindEventtoOnRecoveringfromDamage (EventDispatchers|CreateEvent :!event Custom|OnRecovering))
  (Rendering|Material|SetMaterial (Variables|Default|GetCube) 0 (Variables|Default|GetDynamicMaterial)))

(event EventOnSubComponentOverlap
  (params (OverlappedComponent :type Primitive%20Component%20Object%20Reference) (OtherActor :type Actor%20Object%20Reference) (OtherComp :type Primitive%20Component%20Object%20Reference) (OtherBodyIndex :type Integer) (bFromSweep :type Boolean) (SweepResult :type Hit%20Result%20Structure%20%28by%20ref%29))
  (|CallParentFunction OverlappedComponent OtherActor OtherComp OtherBodyIndex bFromSweep SweepResult))

(event EventOnSubComponentHit
  (params (HitComponent :type Primitive%20Component%20Object%20Reference) (OtherActor :type Actor%20Object%20Reference) (OtherComp :type Primitive%20Component%20Object%20Reference) (NormalImpulse :type Vector :default "0, 0, 0") (Hit :type Hit%20Result%20Structure%20%28by%20ref%29))
  (|CallParentFunction HitComponent OtherActor OtherComp NormalImpulse Hit))

(event EventPossessed
  (params (NewController :type Controller%20Object%20Reference))
  (|CallParentFunction NewController)
  (bind _asplayer_controller (Utilities|Casting|CastToPlayerController NewController))
  (bind _returnvalue (UserInterface|CreateWidget "/Game/Core/UI/HUDWidget.HUDWidget_C" _asplayer_controller))
  (bind _output_get (Variables|Default|SetHudWidget _returnvalue))
  (UserInterface|Viewport|AddtoViewport _output_get 0))

(event EventUnpossessed
  (params (OldController :type Controller%20Object%20Reference))
  (|CallParentFunction OldController)
  (Widget|RemovefromParent (Variables|Default|GetHudWidget))
  (Variables|Default|SetHudWidget 0))

(fn ConstructionScript
  (Transformation|SetRelativeLocation (Variables|Character|GetMesh) (Math|Vector|MakeVector 0.0 0.0 (- 0.0 (Components|Capsule|GetUnscaledCapsuleHalfHeight (Variables|Default|GetCapsuleComponent)))) false false)
  (Transformation|SetRelativeScale3D (Variables|Character|GetMesh) (Math|Vector|MakeVector 2.0 2.0 (/ (* (Components|Capsule|GetUnscaledCapsuleHalfHeight (Variables|Default|GetCapsuleComponent)) 2.0) 25.0)))
  (Transformation|SetRelativeScale3D (Variables|Default|GetCube) (Math|Vector|MakeVector 0.51 0.51 (* (Components|Capsule|GetUnscaledCapsuleHalfHeight (Variables|Default|GetCapsuleComponent)) 0.02))))